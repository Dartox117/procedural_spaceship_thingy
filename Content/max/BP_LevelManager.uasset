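; BP_LevelManager spawns level tiles along the X axis and keeps a rolling window of them.
; Appel_Construction_Tuile spawns the actor class from STTuiles at the given index, offset from Position by DecalageTuile times TailleTuile.
; Each tile joins ListeTuiles, and once the list exceeds ten the oldest is destroyed to free space.
; CheckTuile is an empty stub with unconnected leftover nodes.
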(event Custom|Appel_Construction_Tuile
  (params (Position :type Vector) (TuileNo :type Integer))
  (bind _liste_tuiles (Variables|Default|GetListe_Tuiles))
  (bind _liste_tuiles_2 (Variables|Default|GetListe_Tuiles))
  (bind _returnvalue (Game|SpawnActorfromClass (Utilities|Struct|BreakST_Tuiles (Utilities|Array|Get(acopy) (Variables|Default|GetST_Tuiles) TuileNo)) (Math|Transform|MakeTransform (Math|Vector|MakeVector (+ (* (Variables|Default|GetDecalage_Tuile) (Variables|Default|GetTaille_Tuile)) (.x Position)) (.y Position) (.z Position)) "0, 0, 0" "1.000000,1.000000,1.000000") "Undefined" "MultiplyWithRoot" 0 0))
  (Utilities|Array|Add _liste_tuiles _returnvalue)
  (if (> (Utilities|Array|Length _liste_tuiles) 10)
    (Actor|DestroyActor (Utilities|Array|Get(acopy) _liste_tuiles_2))
    (Utilities|Array|RemoveIndex _liste_tuiles_2)))

(fn ConstructionScript)

(fn CheckTuile
  (params (TuileNo :type Integer) (Vector :type Vector)))